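; Game mode for an anomaly-spotting loop game, scoring a front-or-not choice against whether the current streamed level is a variant.
; BeginPlay loads base level Diff0 and builds the variant name list.
; JudgeChoice counts consecutive correct answers, removes solved variants, and prints StageClear at nine.
; Otherwise it unloads the current level, then randomly either loads a remaining variant or selects Diff0 without loading it.
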(event `self.ReceiveBeginPlay`
  (for _index (range 1 3)
    (`KismetArrayLibrary.Array_Add` (`self.Diff List`) (`KismetStringLibrary.Conv_StringToName` (`KismetStringLibrary.Concat_StrStr` "Diff" (`KismetStringLibrary.Conv_IntToString` _index)))))
  (`GameplayStatics.LoadStreamLevel` "Diff0" true true))

(event `JudgeChoice`
  (params (`Is Front` :type Boolean))
  (bind _returnvalue (`KismetArrayLibrary.Array_Length` (`self.Diff List`)))
  (if (== `Is Front` (`self.Correct Is FFront`))
    (`/Engine/EditorBlueprintResources/StandardMacros.IncrementInt` (`self.Progress Count`)
      (:`  `
        (`KismetArrayLibrary.Array_RemoveItem` (`self.Diff List`) (`self.level Name`))))
    (else
      (set `self.Progress Count` 0)))
  (if (>= (`self.Progress Count`) 9)
    (`KismetSystemLibrary.PrintString` "StageClear")
    (else
      (`GameplayStatics.UnloadStreamLevel` (`self.level Name`) true)
      (bind _output_get (set `self.LevelIndex` (`KismetMathLibrary.RandomInteger` (* _returnvalue 2))))
      (if (< _output_get _returnvalue)
        (set `self.level Name` (`|GetArrayItem` (`self.Diff List`) (`self.LevelIndex`)))
        (set `self.Correct Is FFront` false)
        (`GameplayStatics.LoadStreamLevel` (`self.level Name`) true true)
        (else
          (set `self.level Name` "Diff0")
          (set `self.Correct Is FFront` true))))))

(fn `UserConstructionScript`)