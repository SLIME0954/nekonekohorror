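; BP_warp is a two-way warp that teleports overlapping actors and reports the direction taken to the gamemode as a choice.
; Front sends actors to Back with mirrored offset and the warp's yaw plus 180, calling JudgeChoice(true).
; Back sends them to Front with the same offset, calling JudgeChoice(false).
; An Iswarping flag blocks re-triggering until something overlaps Flagoff; the inverted player velocity is stored but never applied.
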(event `self.front.OnComponentBeginOverlap`
  (params (OverlappedComponent :type "PrimitiveComponent Object Reference") (OtherActor :type "Actor Object Reference") (OtherComp :type "PrimitiveComponent Object Reference") (OtherBodyIndex :type Integer) (bFromSweep :type Boolean) (SweepResult :type "HitResult Structure (by ref)"))
  (bind (_returnvalue_roll _returnvalue_pitch _returnvalue_yaw) (`KismetMathLibrary.BreakRotator` (`self.K2_GetActorRotation`)))
  (bind _returnvalue (`GameplayStatics.GetPlayerPawn` 0))
  ;[1 1 1] Warpシステム
  (if (not (`self.Iswarping`))
    (set `self.Iswarping` true)
    (`self.K2_SetActorLocationAndRotation` OtherActor (+ (* (- (`self.K2_GetActorLocation` OtherActor) (`SceneComponent.K2_GetComponentLocation` (`self.front`))) (-1.0 -1.0 -1.0)) (`SceneComponent.K2_GetComponentLocation` (`self.back`))) (`KismetMathLibrary.MakeRotator` _returnvalue_roll _returnvalue_pitch (+ _returnvalue_yaw 180.0)) false false)
    (`Pawn.AddControllerYawInput` _returnvalue 0.0)
    (set `self.Velocity` (* (`MovementComponent.Velocity` (`Pawn.GetMovementComponent` _returnvalue)) (-1.0 -1.0 -1.0)))
    (bind _asgamemode (cast `/Game/Blueprint/gamemode` (`GameplayStatics.GetGameMode`)))
    (`/Game/Blueprint/gamemode.JudgeChoice` _asgamemode true)))

(event `self.back.OnComponentBeginOverlap`
  (params (OverlappedComponent :type "PrimitiveComponent Object Reference") (OtherActor :type "Actor Object Reference") (OtherComp :type "PrimitiveComponent Object Reference") (OtherBodyIndex :type Integer) (bFromSweep :type Boolean) (SweepResult :type "HitResult Structure (by ref)"))
  ;[1 1 1] Warpシステム
  (if (not (`self.Iswarping`))
    (set `self.Iswarping` true)
    (`self.K2_SetActorLocation` OtherActor (+ (- (`self.K2_GetActorLocation` OtherActor) (`SceneComponent.K2_GetComponentLocation` (`self.back`))) (`SceneComponent.K2_GetComponentLocation` (`self.front`))) false false)
    (bind _asgamemode (cast `/Game/Blueprint/gamemode` (`GameplayStatics.GetGameMode`)))
    (`/Game/Blueprint/gamemode.JudgeChoice` _asgamemode false)))

(event `self.flagoff.OnComponentBeginOverlap`
  (params (OverlappedComponent :type "PrimitiveComponent Object Reference") (OtherActor :type "Actor Object Reference") (OtherComp :type "PrimitiveComponent Object Reference") (OtherBodyIndex :type Integer) (bFromSweep :type Boolean) (SweepResult :type "HitResult Structure (by ref)"))
  ;[1 1 1] warpフラグ管理
  (set `self.Iswarping` false))

(fn `UserConstructionScript`)